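; Drop item manager for ResidentHorror that spawns discarded inventory items in the world and records them per level.
; DropItem spawns the item's class with its slot data, refreshes the inventory and enables mesh physics, unequipping a matching weapon for equippable items.
; New drops are stored in DropItemData by level name and location.
; On BeginPlay, if a save exists, it respawns the level's items from Game Instance data without re-recording them.
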(event `self.ReceiveBeginPlay`
  (bind _returnvalue (`GameplayStatics.DoesSaveGameExist` "ResidentHorrorGlobal"))
  (if _returnvalue
    (bind _retrievergameinstanceresidenthorror (message `/Game/ResidentHorrorV1/Blueprints/BP_SaveLoad/Blueprints/BPI_SavemResidentHorror.RetrieverGameInstanceResidentHorror` (`GameplayStatics.GetGameInstance`)))
    (bind _output_get (set `self.Game Instance Resident Horror` _retrievergameinstanceresidenthorror))
    (bind _drop_item_data (`/Game/ResidentHorrorV1/Blueprints/BP_Core/ResidentHorrorV1_GameInstance.Drop item data` _output_get))
    (set `self.Drop item data` _drop_item_data)
    (bind _returnvalue_2 (`GameplayStatics.GetCurrentLevelName` true))
    (bind _droppeditemsonmap (break `/Game/ResidentHorrorV1/Character/BP_Character/S_DropItemCompound` (`BlueprintMapLibrary.Map_Find` _drop_item_data (`KismetStringLibrary.Conv_StringToName` _returnvalue_2))))
    (bind _keys (`BlueprintMapLibrary.Map_Keys` _droppeditemsonmap))
    (for _array_element _keys
      (bind (_objectclass _objecttransform _slot) (break `/Game/ResidentHorrorV1/Character/BP_Character/S_DropItemData` (`BlueprintMapLibrary.Map_Find` _droppeditemsonmap _array_element)))
      (`self.Drop Item` true _objectclass _slot _array_element))))

(fn `Close Container Inventory`
  (bind _container (`/Game/ResidentHorrorV1/Blueprints/BP_Inventory/BPC_Inventory.Container` (`/Game/ResidentHorrorV1/Character/BP_Character/BP_Resident_HorrorV1.BPC_Inventory` (`/Game/ResidentHorrorV1/Blueprints/BP_FunctionLibray/BPFL_LibrayCharacter.My character Player`)))
    (:`then`
      (bind _bpc_inventorycontainer (`/Game/ResidentHorrorV1/Blueprints/BP_Items/Container/BP_MasterContainer/BP_MasterContainer.BPC_InventoryContainer` _container)
        (:`then`
          (`/Game/ResidentHorrorV1/Blueprints/BP_Inventory/BPC_Inventory.Open/Close Inventory` _bpc_inventorycontainer)
          (set `/Game/ResidentHorrorV1/Blueprints/BP_Items/Container/BP_MasterContainer/BP_MasterContainer.Open Inventory Container?` false _container))
        (:`else`)))
    (:`else`)))

(fn `Drop Item`
  (params (`From Load` :type Boolean) (`Base interact` :type "/Game/ResidentHorrorV1/Blueprints/BP_Inventory/DA_BaseInteract Object Reference") (`Slot Struct` :type "/Game/ResidentHorrorV1/Blueprints/BP_Inventory/S_SlotStruct Structure") (Location :type "Vector Structure"))
  (locals (`Discarded Master Interact` :type "/Game/ResidentHorrorV1/Blueprints/BP_Interact/BP_Master_Interact/BP_Master_Interact Object Reference"))
  (bind _asbp_player (`/Game/ResidentHorrorV1/Blueprints/BP_FunctionLibray/BPFL_LibrayCharacter.My character Player`))
  (bind _asbp_player_2 (`/Game/ResidentHorrorV1/Blueprints/BP_FunctionLibray/BPFL_LibrayCharacter.My character Player`))
  (bind _returnvalue (`KismetMathLibrary.Conv_VectorToTransform` (`local.Location`)))
  (bind _e_interact_viisibility (`/Game/ResidentHorrorV1/Blueprints/BP_Interact/BP_Master_Interact/BP_Master_Interact.E Interact VIisibility` (`local.Discarded Master Interact`)))
  (bind _bpc_inventory (`/Game/ResidentHorrorV1/Character/BP_Character/BP_Resident_HorrorV1.BPC_Inventory` _asbp_player))
  ;[0 0 0 0.5] Discard
  (`|ExecutionSequence`
    (:`then_0`
      ;[0 0 0 0.5] Save Drop Item
      (if (not (`local.From Load`))
        (`self.Save Drop Item` (`local.Location`) _returnvalue (`local.Slot Struct`) `Base interact`)))
    (:`then_1`
      (bind _returnvalue_2 (`|SpawnActorFromClass` (`/Game/ResidentHorrorV1/Blueprints/BP_Inventory/DA_BaseInteract.Master Class` `Base interact`) _returnvalue "Undefined" "MultiplyWithRoot" null null))
      (set `/Game/ResidentHorrorV1/Blueprints/BP_Interact/BP_Master_Interact/BP_Master_Interact.S ItemStrucuture` `Slot Struct` _returnvalue_2)
      (`/Game/ResidentHorrorV1/Blueprints/BP_Inventory/BPC_Inventory.RefreshAllSlot` (`/Game/ResidentHorrorV1/Character/BP_Character/BP_Resident_HorrorV1.BPC_Inventory` _asbp_player))
      (`/Game/ResidentHorrorV1/Blueprints/BP_Inventory/BPC_Inventory.Open/Close Inventory` _bpc_inventory)
      (`/Game/ResidentHorrorV1/Blueprints/BP_Inventory/BPC_Inventory.Open/Close Inventory` _bpc_inventory)
      (bind _output_get (set `local.Discarded Master Interact` _returnvalue_2))
      (if (`/Game/ResidentHorrorV1/Blueprints/BP_Inventory/DA_BaseInteract.Is Equip?` (`.DA_BaseInteract_112_E5D63A474E86D51C38EA9ABF9499DC91` (break `/Game/ResidentHorrorV1/Blueprints/BP_Inventory/S_Item_Structure` (`.ItemStructure_3_D962DD8B4106829899F7C99F3F34F837` (break `/Game/ResidentHorrorV1/Blueprints/BP_Inventory/S_SlotStruct` (`local.Slot Struct`))))))
        ;;[0 0 0] Enable physics when dropping an item with a skeletal mesh. This also applies to weapons that have the “Equip?” variable enabled.
        (`self.Close Container Inventory`)
        (`self.Try Unequip` _output_get)
        (bind _skeletalmesh (`/Game/ResidentHorrorV1/Blueprints/BP_Interact/BP_Master_Interact/BP_Master_Interact.SkeletalMesh` _returnvalue_2))
        (`PrimitiveComponent.SetSimulatePhysics` _skeletalmesh true)
        (`PrimitiveComponent.SetCollisionObjectType` _skeletalmesh "ECC_GameTraceChannel1")
        (bind _wb_hudplayer (`/Game/ResidentHorrorV1/Character/BP_Character/BP_Resident_HorrorV1.WB HudPlayer` _asbp_player_2)
          (:`then`
            (`/Game/ResidentHorrorV1/Blueprints/WBP/WBP_Player/WBP_HudPlayer.Hud Elements Visibility Off` _wb_hudplayer)
            (`/Game/ResidentHorrorV1/Blueprints/BP_Inventory/BPC_Inventory.Open/Close Inventory` (`/Game/ResidentHorrorV1/Character/BP_Character/BP_Resident_HorrorV1.BPC_Inventory` _asbp_player_2))
            (`SceneComponent.SetVisibility` (`/Game/ResidentHorrorV1/Blueprints/BP_Interact/BP_Master_Interact/BP_Master_Interact.OverlayItem` (`local.Discarded Master Interact`)) false false)
            (`PrimitiveComponent.SetCollisionEnabled` (`/Game/ResidentHorrorV1/Blueprints/BP_Interact/BP_Master_Interact/BP_Master_Interact.SkeletalMesh` (`local.Discarded Master Interact`)) "QueryAndPhysics")
            (`PrimitiveComponent.SetCollisionEnabled` (`/Game/ResidentHorrorV1/Blueprints/BP_Interact/BP_Master_Interact/BP_Master_Interact.E Interact VIisibility` (`local.Discarded Master Interact`)) "NoCollision"))
          (:`else`))
        (else
          ;;[0 0 0] Activate physic Item static mesh
          (`PrimitiveComponent.SetSimulatePhysics` (`/Game/ResidentHorrorV1/Blueprints/BP_Interact/BP_Master_Interact/BP_Master_Interact.ItemWorld` _returnvalue_2) true)
          (`PrimitiveComponent.SetCollisionObjectType` (`/Game/ResidentHorrorV1/Blueprints/BP_Interact/BP_Master_Interact/BP_Master_Interact.ItemWorld` (`local.Discarded Master Interact`)) "ECC_GameTraceChannel1")
          (`SceneComponent.SetVisibility` (`/Game/ResidentHorrorV1/Blueprints/BP_Interact/BP_Master_Interact/BP_Master_Interact.OverlayItem` (`local.Discarded Master Interact`)) false false)
          (`PrimitiveComponent.SetCollisionEnabled` _e_interact_viisibility "NoCollision")
          (`PrimitiveComponent.SetCollisionResponseToAllChannels` _e_interact_viisibility "ECR_Ignore"))))))

(fn `Save Drop Item`
  (params (Key :type "Vector Structure (by ref)") (`Object Transform` :type "Transform Structure") (slot :type "/Game/ResidentHorrorV1/Blueprints/BP_Inventory/S_SlotStruct Structure") (`Object class` :type "/Game/ResidentHorrorV1/Blueprints/BP_Inventory/DA_BaseInteract Object Reference"))
  (locals (`Local Compound var` :type "Map of Vector Structure to /Game/ResidentHorrorV1/Character/BP_Character/S_DropItemData Structure"))
  (bind _local_compound_var (`local.Local Compound var`))
  (bind _returnvalue (`GameplayStatics.GetCurrentLevelName` true))
  (bind _returnvalue_2 (`KismetStringLibrary.Conv_StringToName` _returnvalue))
  (set `local.Local Compound var` (`.Droppeditemsonmap_5_B592C6E649FA755C8EFA23B9DA962785` (break `/Game/ResidentHorrorV1/Character/BP_Character/S_DropItemCompound` (`BlueprintMapLibrary.Map_Find` (`self.Drop item data`) _returnvalue_2))))
  (`BlueprintMapLibrary.Map_Add` _local_compound_var Key (make `/Game/ResidentHorrorV1/Character/BP_Character/S_DropItemData` `Object class` `Object Transform` slot))
  (`BlueprintMapLibrary.Map_Add` (`self.Drop item data`) _returnvalue_2 (make `/Game/ResidentHorrorV1/Character/BP_Character/S_DropItemCompound` _local_compound_var)))

(fn `Try Unequip`
  (params (Object :type "Object Object Reference"))
  (bind _asbp_player (`/Game/ResidentHorrorV1/Blueprints/BP_FunctionLibray/BPFL_LibrayCharacter.My character Player`))
  (if (== (`GameplayStatics.GetObjectClass` (`/Game/ResidentHorrorV1/Character/BP_Character/BP_Resident_HorrorV1.Equipped Weapon` _asbp_player)) (`GameplayStatics.GetObjectClass` Object))
    (`/Game/ResidentHorrorV1/Character/BP_Character/BP_Resident_HorrorV1.Unequip Active Weapon` _asbp_player)))