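; Behavior tree task that decides whether an AI keeps attacking its AttackTarget, accounting for players hiding in tall grass.
; A visible player, or a hidden one whose distance plus a small padding is within CheckDistance, makes AI_MasterAI enter its attacking state.
; A hidden player farther away clears the target and switches the AI to random-location state.
; Each branch finishes successfully, but a failed cast never finishes the task.
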(event `self.ReceiveExecuteAI`
  (params (OwnerController :type "AIController Object Reference") (ControlledPawn :type "Pawn Object Reference"))
  (bind _asmy_player_character (cast `MyPlayerCharacter` (`BTFunctionLibrary.GetBlackboardValueAsActor` (`self.AttackTarget`))))
  (if (`MyPlayerCharacter.IsHiddingInTallGrass` _asmy_player_character)
    (if (<= (+ (`KismetMathLibrary.Vector_Distance` (`Actor.K2_GetActorLocation` ControlledPawn) (`Actor.K2_GetActorLocation` (`BTFunctionLibrary.GetBlackboardValueAsActor` (`self.AttackTarget`)))) 50.0) (`self.CheckDistance`))
      (bind _asai_master_ai (cast `/Game/EggContent/AI/Structure/AI_MasterAI` OwnerController))
      (`/Game/EggContent/AI/Structure/AI_MasterAI.SetStateAsAttacking` _asai_master_ai (`BTFunctionLibrary.GetBlackboardValueAsActor` (`self.AttackTarget`)))
      (else
        (`BTFunctionLibrary.ClearBlackboardValue` (`self.AttackTarget`))
        (bind _asai_master_ai_2 (cast `/Game/EggContent/AI/Structure/AI_MasterAI` OwnerController))
        (`/Game/EggContent/AI/Structure/AI_MasterAI.SetStateAsRandomLocation` _asai_master_ai_2)))
    (`self.FinishExecute` true)
    (else
      (bind _asai_master_ai_3 (cast `/Game/EggContent/AI/Structure/AI_MasterAI` OwnerController))
      (`/Game/EggContent/AI/Structure/AI_MasterAI.SetStateAsAttacking` _asai_master_ai_3 (`BTFunctionLibrary.GetBlackboardValueAsActor` (`self.AttackTarget`)))
      (`self.FinishExecute` true))))