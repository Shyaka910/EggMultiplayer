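; Tall-grass volume that hides crouching players from AI sight, evaluated only on the server.
; Sphere overlaps track players inside; each tick, crouch state and head-bone height against the grass decide hiding, which toggles their sight stimulus registration and hiding state.
; A box, sized in construction to fit the sphere's radius and grass height, has query collision switched off while any tracked player stands.
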(event `self.ReceiveBeginPlay`)

(event `self.ReceiveTick`
  (params (DeltaSeconds :type "Float (single-precision)"))
  (bind _box (`self.Box`))
  (`|ExecutionSequence`
    (:`then_0`
      (`/Engine/EditorBlueprintResources/ActorMacros.Switch Has Authority`
        (:`Authority`
          (`self.Check if all actors are crouched`)
          (for _array_element (`self.InBoundPlayers`)
            (bind _charactermovement (`Character.CharacterMovement` _array_element))
            (if (and (<= (`KismetMathLibrary.Abs` (- (.z (.location (`SkinnedMeshComponent.GetBoneTransform` (`Character.Mesh` _array_element) "head" "RTS_World"))) (+ (.z (`BoxComponent.GetUnscaledBoxExtent` _box)) (.z (`SceneComponent.K2_GetComponentLocation` _box))))) (+ (`self.GrassHeight`) (`self.ExposionTolerance`))) (`NavMovementComponent.IsCrouching` _charactermovement))
              (bind _returnvalue (`MyPlayerCharacter.IsHiddingInTallGrass` _array_element))
              (if (not _returnvalue)
                (if (`NavMovementComponent.IsCrouching` _charactermovement) :!label _label
                  (`self.In` _array_element)
                  (else
                    (`self.Out` _array_element :!label _label_2))))
              (elif _returnvalue
                (goto _label_2)
                (else
                  (goto _label))))))))))

(event `self.CollisionComponent.OnComponentBeginOverlap`
  (params (OverlappedComponent :type "PrimitiveComponent Object Reference") (OtherActor :type "Actor Object Reference") (OtherComp :type "PrimitiveComponent Object Reference") (OtherBodyIndex :type Integer) (bFromSweep :type Boolean) (SweepResult :type "HitResult Structure (by ref)"))
  (`/Engine/EditorBlueprintResources/ActorMacros.Switch Has Authority`
    (:`Authority`
      (bind _asmy_player_character (cast `MyPlayerCharacter` OtherActor))
      (`KismetArrayLibrary.Array_AddUnique` (`self.InBoundPlayers`) _asmy_player_character))))

(event `In`
  (params (InActor :type "MyPlayerCharacter Object Reference"))
  (bind _asbp_my_player_character (cast `/Game/EggContent/BP_MyPlayerCharacter` InActor))
  (`AIPerceptionStimuliSourceComponent.UnregisterFromSense` (`/Game/EggContent/BP_MyPlayerCharacter.AIPerceptionStimuliSource` _asbp_my_player_character) "/Script/AIModule.AISense_Sight")
  (`MyPlayerCharacter.SetHiddingInTallGrass` _asbp_my_player_character true)
  (`/Game/EggContent/BP_MyPlayerCharacter.EventOnHidding` _asbp_my_player_character true))

(event `self.CollisionComponent.OnComponentEndOverlap`
  (params (OverlappedComponent :type "PrimitiveComponent Object Reference") (OtherActor :type "Actor Object Reference") (OtherComp :type "PrimitiveComponent Object Reference") (OtherBodyIndex :type Integer))
  (`/Engine/EditorBlueprintResources/ActorMacros.Switch Has Authority`
    (:`Authority`
      (bind _asmy_player_character (cast `MyPlayerCharacter` OtherActor))
      (`self.Out` _asmy_player_character)
      (`PrimitiveComponent.SetCollisionEnabled` (`self.Box`) "QueryOnly")
      (`KismetArrayLibrary.Array_RemoveItem` (`self.InBoundPlayers`) _asmy_player_character))))

(event `Out`
  (params (OutActor :type "MyPlayerCharacter Object Reference"))
  (bind _asbp_my_player_character (cast `/Game/EggContent/BP_MyPlayerCharacter` OutActor))
  (`AIPerceptionStimuliSourceComponent.RegisterForSense` (`/Game/EggContent/BP_MyPlayerCharacter.AIPerceptionStimuliSource` _asbp_my_player_character) "/Script/AIModule.AISense_Sight")
  (`MyPlayerCharacter.SetHiddingInTallGrass` _asbp_my_player_character false)
  (`/Game/EggContent/BP_MyPlayerCharacter.EventOnHidding` _asbp_my_player_character false))

(fn `Check if all actors are crouched`
  (locals (bAllCrouched :type Boolean :default true))
  (for _array_element (`self.InBoundPlayers`)
    (if (not (`NavMovementComponent.IsCrouching` (`Character.CharacterMovement` _array_element)))
      (set `local.bAllCrouched` false)
      (break)))
  (`PrimitiveComponent.SetCollisionEnabled` (`self.Box`) (select `bool` (`local.bAllCrouched`) :`false` "NoCollision" :`true` "QueryOnly" :!type "ECollisionEnabled Enum")))

(fn `UserConstructionScript`
  (bind _assphere_collision (cast `SphereComponent` (`self.CollisionComponent`)))
  (bind _returnvalue (/ (* (`SphereComponent.GetUnscaledSphereRadius` _assphere_collision) (`KismetMathLibrary.Sqrt` 2.0)) 2.0))
  (`BoxComponent.SetBoxExtent` (`self.Box`) (`KismetMathLibrary.MakeVector` _returnvalue _returnvalue (`self.GrassHeight`)) true))