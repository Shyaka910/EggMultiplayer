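; Player HUD Blueprint that keeps the health bar and player UI widgets in sync with gameplay events.
; On BeginPlay it binds to the game state's player-joined event to refresh the control-button widget, and to the controlled pawn's CombatComponent health updates to drive the health widget.
; UpdatePlayerScoreHUD exposes the same player UI refresh as a callable function.
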(event `BindCombatCompEvents`
  (bind _returnvalue (`self.GetComponentByClass` (`Controller.K2_GetPawn` (`self.GetOwningPlayerController`)) "/Script/EggTest.CombatComponent"))
  (`/Engine/EditorBlueprintResources/StandardMacros.IsValid` _returnvalue
    (:`Is Valid`
      (add `CombatComponent.OnHealthUpdated` _returnvalue (delegate `OnHealthUpdated_Event`)))))

(event `self.ReceiveBeginPlay`
  (bind _asbp_my_game_state (cast `/Game/EggContent/BP_MyGameState` (`GameplayStatics.GetGameState`)))
  (add `MyGameState.OnPlayerJoined` _asbp_my_game_state (delegate `OnPlayerJoined_Event_0`))
  (`self.BindCombatCompEvents`))

(event `OnPlayerJoined_Event_0`
  (params (InPlayer :type "MyPlayerState Object Reference"))
  (`/Engine/EditorBlueprintResources/StandardMacros.IsValid` InPlayer
    (:`Is Valid`
      (bind _aswb_control_button (cast `/Game/EggContent/UI/WB_ControlButton` (`self.PlayerHudWidget`)))
      (`/Game/EggContent/UI/WB_ControlButton.UpdatePlayerUI` _aswb_control_button))))

(event `OnHealthUpdated_Event`
  (params (NewHealth :type "Float (single-precision)"))
  (bind _aswb_health (cast `/Game/EggContent/UI/WB_Health` (`self.PlayerHealthWidget`)))
  (`/Game/EggContent/UI/WB_Health.UpdateHealthBar` _aswb_health NewHealth (`CombatComponent.MaxHealth` (`self.GetComponentByClass` (`Controller.K2_GetPawn` (`self.GetOwningPlayerController`)) "/Script/EggTest.CombatComponent"))))

(fn `UpdatePlayerScoreHUD`
  (bind _aswb_control_button (cast `/Game/EggContent/UI/WB_ControlButton` (`self.PlayerHudWidget`)))
  (`/Game/EggContent/UI/WB_ControlButton.UpdatePlayerUI` _aswb_control_button))

(fn `UserConstructionScript`)