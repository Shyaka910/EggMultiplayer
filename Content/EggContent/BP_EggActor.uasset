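; BP_EggActor is an explosive egg whose ExplodeEgg function triggers a blast that damages nearby pawns.
; It reports AI-audible noise and spawns explosion particles and sound, then on authority gathers unique pawns with a sphere trace.
; Each pawn receives the GE_EggDamage gameplay effect if it has an ability system component, plus a damage message scaled by distance from the egg.
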(fn `ExplodeEgg`
  (params (DamageCauser :type "MyPlayerCharacter Object Reference"))
  (locals (HitActors :type "Array of Actor Object Reference"))
  (bind _returnvalue (`self.K2_GetActorLocation`))
  (bind _returnvalue_2 (`self.K2_GetActorLocation`))
  (`AISense_Hearing.ReportNoiseEvent` (`self.K2_GetActorLocation`) 1.0 DamageCauser 2000.0)
  (`GameplayStatics.SpawnEmitterAtLocation` "/Game/StarterContent/Particles/P_Explosion.P_Explosion" _returnvalue (struct) (5.0 5.0 5.0))
  (`GameplayStatics.SpawnSoundAtLocation` "/Game/StarterContent/Audio/Explosion_Cue.Explosion_Cue" _returnvalue (struct) 1.0 1.0 0.0 "/Game/ResidentHorrorV1/Audio/Attenuation/SA_Gun_Attenuation.SA_Gun_Attenuation" null)
  (`/Engine/EditorBlueprintResources/ActorMacros.Switch Has Authority`
    (:`Authority`
      (bind _outhits (`KismetSystemLibrary.SphereTraceMulti` :`Start` _returnvalue_2 :`End` _returnvalue_2 :`Radius` (`self.EggImpactRaduis`) :`TraceChannel` "TraceTypeQuery1" :`DrawTime` 10.0))
      (for _array_element _outhits
        (bind _aspawn (cast `Pawn` (`.HitActor` (`GameplayStatics.BreakHitResult` _array_element))))
        (`KismetArrayLibrary.Array_AddUnique` (`local.HitActors`) _aspawn))
      (for _array_element_2 (`local.HitActors`)
        (bind (_aspawn_2 _bsuccess) (cast `Pawn` _array_element_2 :!pure true))
        (if _bsuccess
          (bind _returnvalue_3 (`AbilitySystemBlueprintLibrary.GetAbilitySystemComponent` _aspawn_2))
          (`/Engine/EditorBlueprintResources/StandardMacros.IsValid` _returnvalue_3
            (:`Is Valid`
              (`AbilitySystemComponent.BP_ApplyGameplayEffectToSelf` :`self` _returnvalue_3 :`GameplayEffectClass` "/Game/EggContent/GAS/GameplayEffect/GE_EggDamage.GE_EggDamage_C"))
            (:`Is Not Valid`
              _))
          (message `/Game/ResidentHorrorV1/Blueprints/BP_Weapon/BP_BaseWeapon/Structure/BPI_DamageWeapon.Event Damage` _aspawn_2 (`KismetMathLibrary.MapRangeClamped` (`KismetMathLibrary.Vector_Distance` (`self.K2_GetActorLocation` _aspawn_2) (`self.K2_GetActorLocation`)) (`self.EggImpactRaduis`) 30.0 (`self.MinDamageRate`) (`self.MaxDamageRate`)) (struct) (`local.DamageCauser`)))))))

(fn `UserConstructionScript`)