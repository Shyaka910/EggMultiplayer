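; Door actor that swings its InteractMesh open or closed when OnDoorToggled fires.
; Opening plays the OpenDoor timeline, scaling MaxOpenAngle by Direction and the curve to set relative yaw, so the swing side follows Direction.
; Closing plays a second timeline that multiplies the mesh's current yaw by its DoorClose curve each update.
; Each toggle stops the opposing timeline before starting its own from the beginning.
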(event `self.OnDoorToggled`
  (params (bOpen :type Boolean) (direction :type Integer))
  (bind _interactmesh (`self.InteractMesh`))
  (bind _interactmesh_2 (`self.InteractMesh`))
  (bind (_relativerotation_roll _relativerotation_pitch _relativerotation_yaw) (`KismetMathLibrary.BreakRotator` (`SceneComponent.RelativeRotation` _interactmesh)))
  (bind (_relativerotation_roll_2 _relativerotation_pitch_2) (`KismetMathLibrary.BreakRotator` (`SceneComponent.RelativeRotation` _interactmesh_2)))
  (if bOpen
    (`|ExecutionSequence`
      (:`then_0`
        (bind (_direction _doorclose) (`Timeline|Timeline` :!via `Stop` :!label _label)
          (:`Update`
            (`SceneComponent.K2_SetRelativeRotation` _interactmesh (`KismetMathLibrary.MakeRotator` _relativerotation_roll _relativerotation_pitch (* _doorclose _relativerotation_yaw)) false false))))
      (:`then_1`
        (bind (_direction_2 _dooropen) (`Timeline|OpenDoor` :!via `PlayFromStart` :!label _label_2)
          (:`Update`
            (`SceneComponent.K2_SetRelativeRotation` _interactmesh_2 (`KismetMathLibrary.MakeRotator` _relativerotation_roll_2 _relativerotation_pitch_2 (* _dooropen (* direction (`self.MaxOpenAngle`)))) false false)))))
    (else
      (`|ExecutionSequence`
        (:`then_0`
          (goto _label_2 :!via `Stop`))
        (:`then_1`
          (goto _label :!via `PlayFromStart`))))))

(fn `UserConstructionScript`)