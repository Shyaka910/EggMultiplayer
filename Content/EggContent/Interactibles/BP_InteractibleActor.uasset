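; BP_InteractibleActor is an interactible actor that shows its Widget based on how close the player is.
; Every Tick it shows the Widget only while the viewing player is between 200 and 600 units away, and hides it otherwise.
; When no valid ViewingPlayer is cached, Tick fetches player pawn 0, so only that player drives visibility.
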(event `self.ReceiveTick`
  (params (DeltaSeconds :type "Float (single-precision)"))
  (bind _viewingplayer (`self.ViewingPlayer`)
    (:`then`
      (bind _returnvalue (`KismetMathLibrary.Vector_Distance` (`self.K2_GetActorLocation` _viewingplayer) (`self.K2_GetActorLocation`)))
      (`SceneComponent.SetVisibility` (`self.Widget`) (and (< _returnvalue 600.0) (> _returnvalue 200.0)) false))
    (:`else`
      (set `self.ViewingPlayer` (`GameplayStatics.GetPlayerPawn` 0)))))

(fn `UserConstructionScript`)