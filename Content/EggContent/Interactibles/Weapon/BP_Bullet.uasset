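; Hitscan bullet actor that resolves a weapon shot against eggs, pawns and scenery.
; On BeginPlay, the authority runs a forward visibility line trace and passes the hit to FireMulti.
; Non-pawn hits spawn impact particles and a fading decal; eggs also explode, credited to the instigator, and are destroyed with authority.
; Pawn hits only spawn blood, as the WeaponActor hit callback is disconnected.
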(event `self.ReceiveBeginPlay`
  (bind _returnvalue (`self.K2_GetActorLocation`))
  (`/Engine/EditorBlueprintResources/ActorMacros.Switch Has Authority`
    (:`Authority`
      (bind (_outhit _returnvalue_2) (`KismetSystemLibrary.LineTraceSingle` _returnvalue (+ _returnvalue (* (`self.GetActorForwardVector`) 10000.0)) "TraceTypeQuery1"))
      (`self.FireMulti` _outhit _returnvalue_2))))

(event `FireMulti`
  (params (HitRes :type "HitResult Structure") (bHit :type Boolean))
  (bind (_bblockinghit _binitialoverlap _time _distance _location _impactpoint _normal _impactnormal _physmat _hitactor) (`GameplayStatics.BreakHitResult` HitRes))
  (bind _returnvalue (`KismetMathLibrary.MakeRotFromZ` _impactnormal))
  (if bHit
    (if (not (`.bSuccess` (cast `Pawn` _hitactor :!pure true)))
      (`GameplayStatics.SpawnEmitterAtLocation` (`self.ImpactParticle`) _location _returnvalue)
      (bind _returnvalue_2 (`GameplayStatics.SpawnDecalAtLocation` "/Game/ResidentHorrorV1/Demo/Materials/M_Decal_Bullet.M_Decal_Bullet" (100.0 10.0 10.0) _location (`KismetMathLibrary.MakeRotFromX` _impactnormal) 4.0))
      (`/Engine/EditorBlueprintResources/StandardMacros.IsValid` _returnvalue_2
        (:`Is Valid`
          (`DecalComponent.SetFadeOut` _returnvalue_2 30.0 4.0 true))
        (:`Is Not Valid`
          _))
      (bind _asbp_egg_actor (cast `/Game/EggContent/BP_EggActor` _hitactor))
      (`/Game/EggContent/BP_EggActor.ExplodeEgg` _asbp_egg_actor (cast `MyPlayerCharacter` (`self.GetInstigator`) :!pure true))
      (bind _ascharacter (cast `Character` (`self.GetInstigator`)))
      (if (`self.HasAuthority` _ascharacter)
        (`self.K2_DestroyActor` _asbp_egg_actor))
      (else
        (`NiagaraFunctionLibrary.SpawnSystemAtLocation` "/Game/ResidentHorrorV1/ParticleEffects/NS_Blood.NS_Blood" _location _returnvalue)))))

(fn `UserConstructionScript`)