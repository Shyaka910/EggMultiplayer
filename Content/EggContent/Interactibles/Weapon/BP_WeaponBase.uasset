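; Base weapon Blueprint that handles the pickup label and networked hit damage.
; While interactable, Tick keeps a label actor attached upright and shows the widget only within a distance band from the local player; otherwise both are cleared.
; Owning-client hits go through an unreliable server RPC, which applies a fire damage GameplayEffect and sends a damage message with a headshot multiplier.
; Firing reports a server-side noise event at the weapon's location.
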(event `InteractInterface.SetCanInteract`
  (params (bInteract :type Boolean))
  (if (not bInteract)
    (`SceneComponent.SetVisibility` (`self.WidgetComp`) false false :!label _label)
    (`SceneComponent.SetVisibility` (`self.Widget`) false false)
    (bind _interactlable (`self.InteractLable`)
      (:`then`
        (`self.K2_DestroyActor` _interactlable))
      (:`else`))))

(event `self.ReceiveTick`
  (params (DeltaSeconds :type "Float (single-precision)"))
  (bind _returnvalue (`InteractInterface.CanInteract`))
  (if _returnvalue
    (`self.InteractLable`
      (:`then`
        _)
      (:`else`
        (bind _returnvalue_2 (`|SpawnActorFromClass` "/Game/EggContent/Interactibles/Weapon/BP_WeaponLable.BP_WeaponLable_C" (`KismetMathLibrary.MakeTransform` (`self.K2_GetActorLocation`)) "Undefined" "MultiplyWithRoot" null null))
        (bind _output_get (set `self.InteractLable` _returnvalue_2))
        (`self.K2_AttachToComponent` _output_get (`self.InteractMesh`) "None" "SnapToTarget" "KeepWorld" "KeepRelative" true)))
    (bind _viewingplayer (`self.ViewingPlayer`)
      (:`then`
        (bind _returnvalue_3 (`KismetMathLibrary.Vector_Distance` (`self.K2_GetActorLocation` _viewingplayer) (`self.K2_GetActorLocation`)))
        (`SceneComponent.SetVisibility` (`self.Widget`) (and (< _returnvalue_3 400.0) (> _returnvalue_3 200.0)) false)
        (`self.K2_SetActorRotation` :`self` (`self.InteractLable`)))
      (:`else`
        (set `self.ViewingPlayer` (`GameplayStatics.GetPlayerPawn` 0))))
    (else
      (goto _label))))

(event `self.OnWeaponFireHit`
  (params (HitPlayer :type "Character Object Reference") (BulletActor :type "Actor Object Reference") (HitRes :type "HitResult Structure (by ref)"))
  (`self.ServerWeaponHit` HitPlayer BulletActor HitRes))

(event `ServerWeaponHit`
  (params (HitPlayer :type "Character Object Reference") (BulletActor :type "Actor Object Reference") (HitRes :type "HitResult Structure (by ref)"))
  (bind _damagerate (`self.DamageRate`))
  (bind (_asmy_player_character _bsuccess) (cast `MyPlayerCharacter` (`self.GetOwner`) :!pure true))
  (if (!= HitPlayer (`self.GetOwner`))
    (`AbilitySystemComponent.BP_ApplyGameplayEffectToTarget` :`self` (`AbilitySystemBlueprintLibrary.GetAbilitySystemComponent` (`self.GetOwner`)) :`GameplayEffectClass` "/Game/EggContent/GAS/GameplayEffect/GE_FireDamage.GE_FireDamage_C" :`Target` (`AbilitySystemBlueprintLibrary.GetAbilitySystemComponent` HitPlayer))
    (if _bsuccess
      (message `/Game/ResidentHorrorV1/Blueprints/BP_Weapon/BP_BaseWeapon/Structure/BPI_DamageWeapon.Event Damage` HitPlayer (`KismetMathLibrary.SelectFloat` (* _damagerate 6.0) _damagerate (== (`.HitBoneName` (`GameplayStatics.BreakHitResult` HitRes)) "head")) HitRes _asmy_player_character))))

(event `self.OnWeaponFired`
  (`AISense_Hearing.ReportNoiseEvent` (`self.K2_GetActorLocation`) 1.0 (`self.GetOwner`) 1000.0))

(fn `UserConstructionScript`)