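; BP_CubeActor is an interactible actor that shows a floating text label to a nearby local player.
; Box overlap begin and end store or clear the overlapping MyPlayerCharacter and toggle TextRender visibility only if that character is locally controlled.
; While a character is stored, Tick turns the text to face the local camera.
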(event `self.ReceiveTick`
  (params (DeltaSeconds :type "Float (single-precision)"))
  (bind _as_my_player_character (`self.As My Player Character`)
    (:`then`
      (if (`Pawn.IsLocallyControlled` _as_my_player_character)
        (`SceneComponent.K2_SetWorldRotation` (`self.TextRender`) (`KismetMathLibrary.FindLookAtRotation` (`self.K2_GetActorLocation`) (`PlayerCameraManager.GetCameraLocation` (`GameplayStatics.GetPlayerCameraManager` 0))) false false)))
    (:`else`)))

(event `self.BoxComp.OnComponentBeginOverlap`
  (params (OverlappedComponent :type "PrimitiveComponent Object Reference") (OtherActor :type "Actor Object Reference") (OtherComp :type "PrimitiveComponent Object Reference") (OtherBodyIndex :type Integer) (bFromSweep :type Boolean) (SweepResult :type "HitResult Structure (by ref)"))
  (bind _asmy_player_character (cast `MyPlayerCharacter` OtherActor))
  (set `self.As My Player Character` _asmy_player_character)
  (if (`Pawn.IsLocallyControlled` _asmy_player_character)
    (`SceneComponent.SetVisibility` (`self.TextRender`) true false)))

(event `self.BoxComp.OnComponentEndOverlap`
  (params (OverlappedComponent :type "PrimitiveComponent Object Reference") (OtherActor :type "Actor Object Reference") (OtherComp :type "PrimitiveComponent Object Reference") (OtherBodyIndex :type Integer))
  (bind _asmy_player_character (cast `MyPlayerCharacter` OtherActor))
  (set `self.As My Player Character` null)
  (if (`Pawn.IsLocallyControlled` _asmy_player_character)
    (`SceneComponent.SetVisibility` (`self.TextRender`) false false)))

(fn `UserConstructionScript`)