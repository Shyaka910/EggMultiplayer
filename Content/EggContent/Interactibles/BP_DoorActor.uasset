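; BP_DoorActor is an interactable swinging door with a widget that shows only while the player pawn is at mid-range.
; Tick caches the player pawn and updates widget visibility from its distance to the door.
; OnDoorToggled starts yaw timelines from near-shut or fully open: opening scales the max angle by direction, closing repeatedly scales the current yaw.
; Construction-script logic for setting an initial open state is disconnected.
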(event `self.ReceiveTick`
  (params (DeltaSeconds :type "Float (single-precision)"))
  (bind _viewingplayer (`self.ViewingPlayer`)
    (:`then`
      (bind _returnvalue (`KismetMathLibrary.Vector_Distance` (`self.K2_GetActorLocation` _viewingplayer) (`self.K2_GetActorLocation`)))
      (`SceneComponent.SetVisibility` (`self.Widget`) (and (< _returnvalue 400.0) (> _returnvalue 200.0)) false))
    (:`else`
      (set `self.ViewingPlayer` (`GameplayStatics.GetPlayerPawn` 0)))))

(event `self.OnDoorToggled`
  (params (bOpen :type Boolean) (direction :type Integer))
  (bind _interactmesh (`self.InteractMesh`))
  (bind _interactmesh_2 (`self.InteractMesh`))
  (bind (_relativerotation_roll _relativerotation_pitch _relativerotation_yaw) (`KismetMathLibrary.BreakRotator` (`SceneComponent.RelativeRotation` _interactmesh_2)))
  (bind (_relativerotation_roll_2 _relativerotation_pitch_2 _relativerotation_yaw_2) (`KismetMathLibrary.BreakRotator` (`SceneComponent.RelativeRotation` (`self.InteractMesh`))))
  (bind (_relativerotation_roll_3 _relativerotation_pitch_3 _relativerotation_yaw_3) (`KismetMathLibrary.BreakRotator` (`SceneComponent.RelativeRotation` (`self.InteractMesh`))))
  (bind (_relativerotation_roll_4 _relativerotation_pitch_4) (`KismetMathLibrary.BreakRotator` (`SceneComponent.RelativeRotation` _interactmesh)))
  (if bOpen
    (`|ExecutionSequence`
      (:`then_1`
        (if (<= (`KismetMathLibrary.Abs` _relativerotation_yaw_3) 1.0)
          (bind (_direction _dooropen) (`Timeline|OpenDoor` :!via `PlayFromStart`)
            (:`Update`
              (`SceneComponent.K2_SetRelativeRotation` _interactmesh (`KismetMathLibrary.MakeRotator` _relativerotation_roll_4 _relativerotation_pitch_4 (* _dooropen (* direction (`self.MaxOpenAngle`)))) false false))))))
    (else
      (`|ExecutionSequence`
        (:`then_1`
          (if (>= (`KismetMathLibrary.Abs` _relativerotation_yaw_2) (`self.MaxOpenAngle`))
            (bind (_direction_2 _doorclose) (`Timeline|Timeline` :!via `PlayFromStart`)
              (:`Update`
                (`SceneComponent.K2_SetRelativeRotation` _interactmesh_2 (`KismetMathLibrary.MakeRotator` _relativerotation_roll _relativerotation_pitch (* _doorclose _relativerotation_yaw)) false false)))))))))

(fn `UserConstructionScript`)