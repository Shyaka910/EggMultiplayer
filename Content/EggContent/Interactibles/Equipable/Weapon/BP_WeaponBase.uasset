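; Base equippable weapon that handles hit damage, egg explosions, firing noise and its pickup label.
; Owning-client hits go by unreliable server RPC to apply a fire damage GameplayEffect and send a damage message, boosted for headshots.
; Egg hits route through server and multicast events to explode the egg, and server-side firing reports noise.
; Tick spawns an attached, fixed-rotation label while interactable and destroys it otherwise.
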(event `self.ReceiveBeginPlay`
  (add `self.OnWeaponHitTarget` (delegate `OnWeaponHitTarget_Event`)))

(event `OnWeaponHitTarget_Event` :!signature `self.OnWeaponHitTarget`
  (params (TargetActor :type "Actor Object Reference") (IsHeadShoot :type Boolean))
  (bind _asbp_egg_actor (cast `/Game/EggContent/BP_EggActor` TargetActor))
  (`self.TriggerServerEggExplosion` _asbp_egg_actor))

(event `TriggerServerEggExplosion`
  (params (Egg :type "/Game/EggContent/BP_EggActor Object Reference"))
  (`self.TriggerMulticastEggExplosion` Egg))

(event `TriggerMulticastEggExplosion`
  (params (Egg :type "/Game/EggContent/BP_EggActor Object Reference"))
  (bind _asmy_player_character (cast `MyPlayerCharacter` (`self.GetOwner`)))
  (`/Game/EggContent/BP_EggActor.ExplodeEgg` Egg _asmy_player_character))

(event `InteractInterface.SetCanInteract`
  (params (bInteract :type Boolean))
  (if (not bInteract)
    (`SceneComponent.SetVisibility` (`self.WidgetComp`) false false :!label _label)
    (bind _interactlable (`self.InteractLable`)
      (:`then`
        (`self.K2_DestroyActor` _interactlable))
      (:`else`))))

(event `self.ReceiveTick`
  (params (DeltaSeconds :type "Float (single-precision)"))
  (bind _returnvalue (`InteractInterface.CanInteract`))
  (if _returnvalue
    (`self.InteractLable`
      (:`then`
        _)
      (:`else`
        (bind _returnvalue_2 (`|SpawnActorFromClass` "/Game/EggContent/Interactibles/Equipable/Weapon/BP_WeaponLable.BP_WeaponLable_C" (`KismetMathLibrary.MakeTransform` (`self.K2_GetActorLocation`)) "Undefined" "MultiplyWithRoot" null null))
        (bind _output_get (set `self.InteractLable` _returnvalue_2))
        (`self.K2_AttachToComponent` _output_get (`self.InteractMesh`) "None" "SnapToTarget" "KeepWorld" "KeepRelative" true)))
    (`self.K2_SetActorRotation` :`self` (`self.InteractLable`))
    (else
      (goto _label))))

(event `self.OnWeaponFireHit`
  (params (HitPlayer :type "Character Object Reference") (BulletActor :type "Actor Object Reference") (HitRes :type "HitResult Structure (by ref)"))
  (`self.ServerWeaponHit` HitPlayer BulletActor HitRes))

(event `ServerWeaponHit`
  (params (HitPlayer :type "Character Object Reference") (BulletActor :type "Actor Object Reference") (HitRes :type "HitResult Structure (by ref)"))
  (bind _damagerate (`self.DamageRate`))
  (bind (_asmy_player_character _bsuccess) (cast `MyPlayerCharacter` (`self.GetOwner`) :!pure true))
  (if (!= HitPlayer (`self.GetOwner`))
    (`AbilitySystemComponent.BP_ApplyGameplayEffectToTarget` :`self` (`AbilitySystemBlueprintLibrary.GetAbilitySystemComponent` (`self.GetOwner`)) :`GameplayEffectClass` "/Game/EggContent/GAS/GameplayEffect/GE_FireDamage.GE_FireDamage_C" :`Target` (`AbilitySystemBlueprintLibrary.GetAbilitySystemComponent` HitPlayer))
    (if _bsuccess
      (message `/Game/ResidentHorrorV1/Blueprints/BP_Weapon/BP_BaseWeapon/Structure/BPI_DamageWeapon.Event Damage` HitPlayer (`KismetMathLibrary.SelectFloat` (* _damagerate 6.0) _damagerate (== (`.HitBoneName` (`GameplayStatics.BreakHitResult` HitRes)) "head")) HitRes _asmy_player_character))))

(event `self.OnWeaponFired`
  (`AISense_Hearing.ReportNoiseEvent` (`self.K2_GetActorLocation`) 1.0 (`self.GetOwner`) 1000.0))

(fn `UserConstructionScript`)