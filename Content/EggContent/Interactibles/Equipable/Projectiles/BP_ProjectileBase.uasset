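; BP_ProjectileBase is a base Blueprint for equipable projectile interactibles that manages a floating label indicating when the projectile can be interacted with.
; Tick polls CanInteract, lazily spawns a BP_ProjectileLable attached to InteractMesh, and resets its world rotation each frame so it stays unrotated.
; When interaction is unavailable, Tick and SetCanInteract share a cleanup path that hides WidgetComp and destroys the label.
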(event `InteractInterface.SetCanInteract`
  (params (bInteract :type Boolean))
  (if (not bInteract)
    (`SceneComponent.SetVisibility` (`self.WidgetComp`) false false :!label _label)
    (bind _interactlable (`self.InteractLable`)
      (:`then`
        (`self.K2_DestroyActor` _interactlable))
      (:`else`))))

(event `self.ReceiveTick`
  (params (DeltaSeconds :type "Float (single-precision)"))
  (bind _returnvalue (`InteractInterface.CanInteract`))
  (if _returnvalue
    (`self.InteractLable`
      (:`then`
        _)
      (:`else`
        (bind _returnvalue_2 (`|SpawnActorFromClass` "/Game/EggContent/Interactibles/Equipable/Weapon/BP_ProjectileLable.BP_ProjectileLable_C" (`KismetMathLibrary.MakeTransform` (`self.K2_GetActorLocation`)) "Undefined" "MultiplyWithRoot" null null))
        (bind _output_get (set `self.InteractLable` _returnvalue_2))
        (`self.K2_AttachToComponent` _output_get (`self.InteractMesh`) "None" "SnapToTarget" "KeepWorld" "KeepRelative" true)))
    (`self.K2_SetActorRotation` :`self` (`self.InteractLable`))
    (else
      (goto _label))))

(fn `UserConstructionScript`)