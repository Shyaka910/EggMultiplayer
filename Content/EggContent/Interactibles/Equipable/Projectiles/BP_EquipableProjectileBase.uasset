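; Base equippable throwable: players pick it up, aim and throw it, and its impacts report noise and play a sound.
; Tick maintains an attached pickup label and, for the local owner while aiming, draws the predicted path with debug spheres.
; Fire sets projectile velocity locally, then through server and multicast events, with the server dropping it from the character.
; Becoming interactable re-enables mesh physics, delayed briefly after throws.
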(event `Fall`
  (if (`self.bIsThrown`)
    (`KismetSystemLibrary.Delay` 0.2)
    (`PrimitiveComponent.SetSimulatePhysics` (`self.InteractMesh`) true)
    (set `self.bIsThrown` false)
    (else
      (`PrimitiveComponent.SetSimulatePhysics` (`self.InteractMesh`) true)
      (set `self.bIsThrown` false))))

(event `InteractInterface.SetCanInteract`
  (params (bInteract :type Boolean))
  (`parent.SetCanInteract` bInteract)
  (if bInteract
    (`self.Fall`)
    (else
      (`SceneComponent.SetVisibility` (`self.WidgetComp`) false false :!label _label)
      (bind _interactlable (`self.InteractLable`)
        (:`then`
          (`self.K2_DestroyActor` _interactlable)
          (set `self.bIsThrown` false))
        (:`else`)))))

(event `self.ReceiveTick`
  (params (DeltaSeconds :type "Float (single-precision)"))
  (bind _owningpawn (`self.OwningPawn`))
  (bind _returnvalue (not (`KismetSystemLibrary.IsValid` (`self.InteractLable`))))
  (`|ExecutionSequence`
    (:`then_0`
      (bind _returnvalue_2 (`InteractInterface.CanInteract`))
      (if _returnvalue_2
        (`self.InteractLable`
          (:`then`
            _)
          (:`else`
            (bind _returnvalue_3 (`|SpawnActorFromClass` "/Game/EggContent/Interactibles/Equipable/Weapon/BP_ProjectileLable.BP_ProjectileLable_C" (`KismetMathLibrary.MakeTransform` (`self.K2_GetActorLocation`)) "Undefined" "MultiplyWithRoot" null null))
            (bind _output_get (set `self.InteractLable` _returnvalue_3))
            (`self.SetActorHiddenInGame` _output_get (`self.bIsThrown`))
            (`self.K2_AttachToComponent` _output_get (`self.InteractMesh`) "None" "SnapToTarget" "KeepWorld" "KeepRelative" true)))
        (`self.K2_SetActorRotation` :`self` (`self.InteractLable`))
        (else
          (goto _label))))
    (:`then_1`
      (`/Engine/EditorBlueprintResources/StandardMacros.IsValid` _owningpawn
        (:`Is Valid`
          (`SceneComponent.SetVisibility` (`self.ThrowIndicatorWidget`) (or (`KismetSystemLibrary.IsValid` (`self.GetOwner`)) (select `bool` _returnvalue :`false` (`Actor.bHidden` (`self.InteractLable`)) :`true` _returnvalue)) false)
          (if (`Pawn.IsLocallyControlled` _owningpawn)
            (bind _returnvalue_4 (`InteractInterface.CanInteract`))
            (if _returnvalue_4
              (set `self.bIsAiming` false)
              (elif (`self.bIsAiming`)
                (bind (_outhit _outpathpositions) (`GameplayStatics.Blueprint_PredictProjectilePath_ByTraceChannel` (`self.K2_GetActorLocation`) (`self.GetAimVelocity`) true (`.SphereRadius` (`KismetSystemLibrary.GetComponentBounds` (`self.InteractMesh`))) "ECC_WorldDynamic" true (`|MakeArray` (`self.GetOwner`) self :!type "Actor Object Reference")))
                (for (_array_element _array_index) _outpathpositions
                  (bind _returnvalue_5 (== (+ _array_index 1) (`KismetArrayLibrary.Array_Length` _outpathpositions)))
                  (`KismetSystemLibrary.DrawDebugSphere` _array_element (/ (`.SphereRadius` (`KismetSystemLibrary.GetComponentBounds` (`self.InteractMesh`))) (`KismetMathLibrary.SelectFloat` 1.0 2.0 _returnvalue_5)) 12 (`KismetMathLibrary.SelectColor` (struct :`R` 0.2 :`B` 1.0 :`A` 1.0) (struct :`R` 1.0 :`G` 1.0 :`B` 1.0 :`A` 1.0) _returnvalue_5) 0.0 (`KismetMathLibrary.SelectFloat` 3.0 0.0 _returnvalue_5)))))))))))

(event `Fire`
  (bind _returnvalue (`self.GetAimVelocity`))
  (`self.ServerLaunch` _returnvalue)
  (set `MovementComponent.Velocity` _returnvalue (`self.ProjectileMovement`))
  (set `self.bIsThrown` true))

(event `ServerLaunch`
  (params (Velocity :type "Vector Structure"))
  (bind _projectilemovement (`self.ProjectileMovement`))
  (set `MovementComponent.Velocity` Velocity _projectilemovement)
  (`ActorComponent.Activate` _projectilemovement false)
  (`self.MulticastLaunch` Velocity)
  (bind _asmy_player_character (cast `MyPlayerCharacter` (`self.GetOwner`)))
  (`MyPlayerCharacter.DropEquippedActor` _asmy_player_character)
  (set `self.bIsThrown` true))

(event `MulticastLaunch`
  (params (Velocity :type "Vector Structure"))
  (set `MovementComponent.Velocity` Velocity (`self.ProjectileMovement`))
  (set `self.bIsThrown` true))

(event `StartAiming`
  (set `self.bIsAiming` true))

(event `StopAiming`
  (set `self.bIsAiming` false))

(event `self.OnInteract`
  (params (InteractingPlayer :type "Pawn Object Reference"))
  (`parent.OnInteract` InteractingPlayer)
  (set `self.OwningPawn` InteractingPlayer)
  (`ActorComponent.SetActive` (`self.ProjectileMovement`) false false))

(event `self.InteractMesh.OnComponentHit`
  (params (HitComponent :type "PrimitiveComponent Object Reference") (OtherActor :type "Actor Object Reference") (OtherComp :type "PrimitiveComponent Object Reference") (NormalImpulse :type "Vector Structure") (Hit :type "HitResult Structure (by ref)"))
  (bind _returnvalue (`self.K2_GetActorLocation`))
  (`/Engine/EditorBlueprintResources/StandardMacros.DoOnce` false :!label _label_2
    (:`Completed`
      (`AISense_Hearing.ReportNoiseEvent` _returnvalue 1.0 (`self.OwningPawn`) 1000.0)
      (`GameplayStatics.PlaySoundAtLocation` "/Game/ResidentHorrorV1/Audio/CharactersAudio/WaveFiles/Foley/Concrete/Walk/CUE_Foley_fs_1p_sneaker_concrete_walk_04_Cue.CUE_Foley_fs_1p_sneaker_concrete_walk_04_Cue" _returnvalue (struct) 1.0 1.0 0.0 "/Game/ResidentHorrorV1/Audio/Attenuation/SA_ProjectileImpact_att.SA_ProjectileImpact_att" null null null)
      (`KismetSystemLibrary.Delay` 2.0)
      (bind _interactlable (`self.InteractLable`)
        (:`then`
          (`self.SetActorHiddenInGame` _interactlable false)
          (set `self.bIsThrown` false)
          (goto _label_2 :!via `Reset`))
        (:`else`)))))

(fn `UserConstructionScript`)