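; BP_Ammo is an interactable ammo pickup that adds bullets to the weapon the interacting player has equipped.
; On interact, it casts to the player character and its equipped WeaponActor, exiting if either fails, then calls AddBullets before any authority check.
; Only on authority, it triggers Reload when the weapon's bullet count then equals the pickup amount, then destroys itself.
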(event `self.OnInteract`
  (params (InteractingPlayer :type "Pawn Object Reference"))
  (bind _bulletscount (`self.BulletsCount`))
  (bind _asbp_my_player_character (cast `/Game/EggContent/BP_MyPlayerCharacter` InteractingPlayer))
  (bind _asweapon_actor (cast `WeaponActor` (`MyPlayerCharacter.CurrentEquippedActor` _asbp_my_player_character)))
  (`WeaponActor.AddBullets` _asweapon_actor _bulletscount)
  (`/Engine/EditorBlueprintResources/ActorMacros.Switch Has Authority`
    (:`Authority`
      (if (<= (`KismetMathLibrary.Abs_Int` (- (`WeaponActor.CurrentBulletsCount` _asweapon_actor) _bulletscount)) 0)
        (`/Game/EggContent/BP_MyPlayerCharacter.Reload` _asbp_my_player_character))
      (`self.K2_DestroyActor`))))

(fn `UserConstructionScript`
  (`parent.UserConstructionScript`))